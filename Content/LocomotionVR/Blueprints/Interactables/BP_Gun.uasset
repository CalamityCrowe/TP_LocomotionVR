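; BP_Gun is a grabbable VR weapon that fires from the hand holding its GripPoint.
; Grabbing enables input and adds that hand's weapon mapping context, while dropping disables and removes it.
; Left and right shoot inputs check the holding hand before calling OnFire, which is defined outside these graphs.
; When UseProjectiles is off, each shot also spawns a VRLine_Render effect from MuzzlePoint to EndPoint.
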(event OnGrabbed(GripPoint)
  ;[1 1 1] Adding the mapping context for when the weapon is grabbed
  (Input|EnableInput (Game|GetPlayerController 0))
  (Input|AddMappingContext (PlayerController|LocalPlayerSubsystems|GetEnhancedInputLocalPlayerSubsystem (Game|GetPlayerController 0)) (select (Utilities|Enum|Equal(Enum) (Class|VRGrabComponent|GetHeldbyHand (Variables|Default|GetGripPoint)) "Right") "/Game/LocomotionVR/Blueprints/Inputs/Contexts/IMC_Weapon_Right.IMC_Weapon_Right" "/Game/LocomotionVR/Blueprints/Inputs/Contexts/IMC_Weapon_Left.IMC_Weapon_Left") 1 "(bIgnoreAllPressedKeysUntilRelease=True,bForceImmediately=False,bNotifyUserSettings=False)"))

(event OnDropped(GripPoint)
  ;[1 1 1] Adding the mapping context for when the weapon is grabbed
  (Input|DisableInput (Game|GetPlayerController 0))
  (Input|RemoveMappingContext (PlayerController|LocalPlayerSubsystems|GetEnhancedInputLocalPlayerSubsystem (Game|GetPlayerController 0)) (select (Utilities|Enum|Equal(Enum) (Class|VRGrabComponent|GetHeldbyHand (Variables|Default|GetGripPoint)) "Right") "/Game/LocomotionVR/Blueprints/Inputs/Contexts/IMC_Weapon_Right.IMC_Weapon_Right" "/Game/LocomotionVR/Blueprints/Inputs/Contexts/IMC_Weapon_Left.IMC_Weapon_Left") "(bIgnoreAllPressedKeysUntilRelease=True,bForceImmediately=False,bNotifyUserSettings=False)"))

(event Input|EnhancedActionEvents|EnhancedInputActionIA_Shoot_Left
  (params (ActionValue :type Boolean) (ElapsedSeconds :type Float%20%28double-precision%29) (TriggeredSeconds :type Float%20%28double-precision%29) (InputAction :type Input%20Action%20Object%20Reference :default "/Game/LocomotionVR/Blueprints/Inputs/Actions/Interact/IA_Shoot_Left.IA_Shoot_Left"))
  (bind _muzzlepoint (Variables|Default|GetMuzzlePoint))
  (:Started
    (if (Utilities|Enum|Equal(Enum) (Class|VRGrabComponent|GetHeldbyHand (Variables|Default|GetGripPoint)) "Left")
      (Class|GrabbableGun|OnFire)
      (if (not (Variables|Default|GetbUseProjectiles))
        (bind _returnvalue (Niagara|SpawnSystematLocation "/Game/LocomotionVR/Niagara/VRLine_Render.VRLine_Render" (Transformation|GetWorldLocation _muzzlepoint) (Transformation|GetWorldRotation _muzzlepoint)))
        (Niagara|SetNiagaraVariable(Vector3) _returnvalue "EndPoint" (Variables|Default|GetEndPoint))))))

(event Input|EnhancedActionEvents|EnhancedInputActionIA_Shoot_Right
  (params (ActionValue :type Boolean) (ElapsedSeconds :type Float%20%28double-precision%29) (TriggeredSeconds :type Float%20%28double-precision%29) (InputAction :type Input%20Action%20Object%20Reference :default "/Game/LocomotionVR/Blueprints/Inputs/Actions/Interact/IA_Shoot_Right.IA_Shoot_Right"))
  (bind _muzzlepoint (Variables|Default|GetMuzzlePoint))
  (:Started
    (if (Utilities|Enum|Equal(Enum) (Class|VRGrabComponent|GetHeldbyHand (Variables|Default|GetGripPoint)) "Right")
      (Class|GrabbableGun|OnFire)
      (if (not (Variables|Default|GetbUseProjectiles))
        (bind _returnvalue (Niagara|SpawnSystematLocation "/Game/LocomotionVR/Niagara/VRLine_Render.VRLine_Render" (Transformation|GetWorldLocation _muzzlepoint) (Transformation|GetWorldRotation _muzzlepoint)))
        (Niagara|SetNiagaraVariable(Vector3) _returnvalue "EndPoint" (Variables|Default|GetEndPoint))))))

(fn ConstructionScript)