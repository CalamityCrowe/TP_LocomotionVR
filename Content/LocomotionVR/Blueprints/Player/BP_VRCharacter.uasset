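; VR player character that initializes headset tracking and animates the left and right hand meshes from controller input.
; On BeginPlay with an HMD enabled, it sets Stage tracking origin and sets pixel density through a console command.
; Enhanced Input actions write pose alphas on each hand's ABP_MannequinsXR instance.
; Grasp and index curl pass analog values through, while point and thumb-up toggle inversely, zero on start or cancel and one on completion.
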(event Input|EnhancedActionEvents|EnhancedInputActionIA_Hand_Grasp_Left
  (params (ActionValue :type Float%20%28double-precision%29) (ElapsedSeconds :type Float%20%28double-precision%29) (TriggeredSeconds :type Float%20%28double-precision%29) (InputAction :type Input%20Action%20Object%20Reference :default "/Game/LocomotionVR/Blueprints/Inputs/Actions/Hands/IA_Hand_Grasp_Left.IA_Hand_Grasp_Left"))
  (bind _lefthand (Variables|Default|GetLeftHand))
  (bind _returnvalue (Components|SkeletalMesh|GetAnimInstance _lefthand))
  ;[1 1 1] Hand Animations
  (:Triggered
    (bind _asabp_mannequins_xr (Utilities|Casting|CastToABP_MannequinsXR _returnvalue))
    (Variables|/Game/LocomotionVR/Characters/MannequinsXR/Meshes/ABP_MannequinsXR.ABP_MannequinsXR_C|SetPoseAlphaGrasp _asabp_mannequins_xr ActionValue))
  (:Canceled
    (bind _asabp_mannequins_xr_2 (Utilities|Casting|CastToABP_MannequinsXR _returnvalue :!label _label))
    (Variables|/Game/LocomotionVR/Characters/MannequinsXR/Meshes/ABP_MannequinsXR.ABP_MannequinsXR_C|SetPoseAlphaGrasp _asabp_mannequins_xr_2 ActionValue))
  (:Completed
    (goto _label)))

(event Input|EnhancedActionEvents|EnhancedInputActionIA_Hand_Point_Left
  (params (ActionValue :type Float%20%28double-precision%29) (ElapsedSeconds :type Float%20%28double-precision%29) (TriggeredSeconds :type Float%20%28double-precision%29) (InputAction :type Input%20Action%20Object%20Reference :default "/Game/LocomotionVR/Blueprints/Inputs/Actions/Hands/IA_Hand_Point_Left.IA_Hand_Point_Left"))
  (bind _lefthand (Variables|Default|GetLeftHand))
  ;[1 1 1] Hand Animations
  (:Started
    (bind _asabp_mannequins_xr (Utilities|Casting|CastToABP_MannequinsXR (Components|SkeletalMesh|GetAnimInstance _lefthand) :!label _label))
    (Variables|/Game/LocomotionVR/Characters/MannequinsXR/Meshes/ABP_MannequinsXR.ABP_MannequinsXR_C|SetPoseAlphaPoint _asabp_mannequins_xr 0.0))
  (:Canceled
    (goto _label))
  (:Completed
    (bind _asabp_mannequins_xr_2 (Utilities|Casting|CastToABP_MannequinsXR (Components|SkeletalMesh|GetAnimInstance _lefthand)))
    (Variables|/Game/LocomotionVR/Characters/MannequinsXR/Meshes/ABP_MannequinsXR.ABP_MannequinsXR_C|SetPoseAlphaPoint _asabp_mannequins_xr_2 1.0)))

(event Input|EnhancedActionEvents|EnhancedInputActionIA_Hand_ThumbUp_Left
  (params (ActionValue :type Float%20%28double-precision%29) (ElapsedSeconds :type Float%20%28double-precision%29) (TriggeredSeconds :type Float%20%28double-precision%29) (InputAction :type Input%20Action%20Object%20Reference :default "/Game/LocomotionVR/Blueprints/Inputs/Actions/Hands/IA_Hand_ThumbUp_Left.IA_Hand_ThumbUp_Left"))
  (bind _lefthand (Variables|Default|GetLeftHand))
  ;[1 1 1] Hand Animations
  (:Started
    (bind _asabp_mannequins_xr (Utilities|Casting|CastToABP_MannequinsXR (Components|SkeletalMesh|GetAnimInstance _lefthand) :!label _label))
    (Variables|/Game/LocomotionVR/Characters/MannequinsXR/Meshes/ABP_MannequinsXR.ABP_MannequinsXR_C|SetPoseAlphaThumbUp _asabp_mannequins_xr 0.0))
  (:Canceled
    (goto _label))
  (:Completed
    (bind _asabp_mannequins_xr_2 (Utilities|Casting|CastToABP_MannequinsXR (Components|SkeletalMesh|GetAnimInstance _lefthand)))
    (Variables|/Game/LocomotionVR/Characters/MannequinsXR/Meshes/ABP_MannequinsXR.ABP_MannequinsXR_C|SetPoseAlphaThumbUp _asabp_mannequins_xr_2 1.0)))

(event Input|EnhancedActionEvents|EnhancedInputActionIA_Hand_IndexCurl_Right
  (params (ActionValue :type Float%20%28double-precision%29) (ElapsedSeconds :type Float%20%28double-precision%29) (TriggeredSeconds :type Float%20%28double-precision%29) (InputAction :type Input%20Action%20Object%20Reference :default "/Game/LocomotionVR/Blueprints/Inputs/Actions/Hands/IA_Hand_IndexCurl_Right.IA_Hand_IndexCurl_Right"))
  (bind _righthand (Variables|Default|GetRightHand))
  (bind _returnvalue (Components|SkeletalMesh|GetAnimInstance _righthand))
  ;[1 1 1] Hand Animations
  (:Triggered
    (bind _asabp_mannequins_xr (Utilities|Casting|CastToABP_MannequinsXR _returnvalue))
    (Variables|/Game/LocomotionVR/Characters/MannequinsXR/Meshes/ABP_MannequinsXR.ABP_MannequinsXR_C|SetPoseAlphaIndexCurl _asabp_mannequins_xr ActionValue))
  (:Canceled
    (bind _asabp_mannequins_xr_2 (Utilities|Casting|CastToABP_MannequinsXR _returnvalue :!label _label))
    (Variables|/Game/LocomotionVR/Characters/MannequinsXR/Meshes/ABP_MannequinsXR.ABP_MannequinsXR_C|SetPoseAlphaIndexCurl _asabp_mannequins_xr_2 ActionValue))
  (:Completed
    (goto _label)))

(event Input|EnhancedActionEvents|EnhancedInputActionIA_Hand_Grasp_Right
  (params (ActionValue :type Float%20%28double-precision%29) (ElapsedSeconds :type Float%20%28double-precision%29) (TriggeredSeconds :type Float%20%28double-precision%29) (InputAction :type Input%20Action%20Object%20Reference :default "/Game/LocomotionVR/Blueprints/Inputs/Actions/Hands/IA_Hand_Grasp_Right.IA_Hand_Grasp_Right"))
  (bind _righthand (Variables|Default|GetRightHand))
  (bind _returnvalue (Components|SkeletalMesh|GetAnimInstance _righthand))
  ;[1 1 1] Hand Animations
  (:Triggered
    (bind _asabp_mannequins_xr (Utilities|Casting|CastToABP_MannequinsXR _returnvalue))
    (Variables|/Game/LocomotionVR/Characters/MannequinsXR/Meshes/ABP_MannequinsXR.ABP_MannequinsXR_C|SetPoseAlphaGrasp _asabp_mannequins_xr ActionValue))
  (:Canceled
    (bind _asabp_mannequins_xr_2 (Utilities|Casting|CastToABP_MannequinsXR _returnvalue :!label _label))
    (Variables|/Game/LocomotionVR/Characters/MannequinsXR/Meshes/ABP_MannequinsXR.ABP_MannequinsXR_C|SetPoseAlphaGrasp _asabp_mannequins_xr_2 ActionValue))
  (:Completed
    (goto _label)))

(event Input|EnhancedActionEvents|EnhancedInputActionIA_Hand_IndexCurl_Left
  (params (ActionValue :type Float%20%28double-precision%29) (ElapsedSeconds :type Float%20%28double-precision%29) (TriggeredSeconds :type Float%20%28double-precision%29) (InputAction :type Input%20Action%20Object%20Reference :default "/Game/LocomotionVR/Blueprints/Inputs/Actions/Hands/IA_Hand_IndexCurl_Left.IA_Hand_IndexCurl_Left"))
  (bind _lefthand (Variables|Default|GetLeftHand))
  (bind _returnvalue (Components|SkeletalMesh|GetAnimInstance _lefthand))
  ;[1 1 1] Hand Animations
  (:Triggered
    (bind _asabp_mannequins_xr (Utilities|Casting|CastToABP_MannequinsXR _returnvalue))
    (Variables|/Game/LocomotionVR/Characters/MannequinsXR/Meshes/ABP_MannequinsXR.ABP_MannequinsXR_C|SetPoseAlphaIndexCurl _asabp_mannequins_xr ActionValue))
  (:Canceled
    (bind _asabp_mannequins_xr_2 (Utilities|Casting|CastToABP_MannequinsXR _returnvalue :!label _label))
    (Variables|/Game/LocomotionVR/Characters/MannequinsXR/Meshes/ABP_MannequinsXR.ABP_MannequinsXR_C|SetPoseAlphaIndexCurl _asabp_mannequins_xr_2 ActionValue))
  (:Completed
    (goto _label)))

(event Input|EnhancedActionEvents|EnhancedInputActionIA_Hand_ThumbUp_Right
  (params (ActionValue :type Float%20%28double-precision%29) (ElapsedSeconds :type Float%20%28double-precision%29) (TriggeredSeconds :type Float%20%28double-precision%29) (InputAction :type Input%20Action%20Object%20Reference :default "/Game/LocomotionVR/Blueprints/Inputs/Actions/Hands/IA_Hand_ThumbUp_Right.IA_Hand_ThumbUp_Right"))
  (bind _righthand (Variables|Default|GetRightHand))
  ;[1 1 1] Hand Animations
  (:Started
    (bind _asabp_mannequins_xr (Utilities|Casting|CastToABP_MannequinsXR (Components|SkeletalMesh|GetAnimInstance _righthand) :!label _label))
    (Variables|/Game/LocomotionVR/Characters/MannequinsXR/Meshes/ABP_MannequinsXR.ABP_MannequinsXR_C|SetPoseAlphaThumbUp _asabp_mannequins_xr 0.0))
  (:Canceled
    (goto _label))
  (:Completed
    (bind _asabp_mannequins_xr_2 (Utilities|Casting|CastToABP_MannequinsXR (Components|SkeletalMesh|GetAnimInstance _righthand)))
    (Variables|/Game/LocomotionVR/Characters/MannequinsXR/Meshes/ABP_MannequinsXR.ABP_MannequinsXR_C|SetPoseAlphaThumbUp _asabp_mannequins_xr_2 1.0)))

(event Input|EnhancedActionEvents|EnhancedInputActionIA_Hand_Point_Right
  (params (ActionValue :type Float%20%28double-precision%29) (ElapsedSeconds :type Float%20%28double-precision%29) (TriggeredSeconds :type Float%20%28double-precision%29) (InputAction :type Input%20Action%20Object%20Reference :default "/Game/LocomotionVR/Blueprints/Inputs/Actions/Hands/IA_Hand_Point_Right.IA_Hand_Point_Right"))
  (bind _righthand (Variables|Default|GetRightHand))
  ;[1 1 1] Hand Animations
  (:Started
    (bind _asabp_mannequins_xr (Utilities|Casting|CastToABP_MannequinsXR (Components|SkeletalMesh|GetAnimInstance _righthand) :!label _label))
    (Variables|/Game/LocomotionVR/Characters/MannequinsXR/Meshes/ABP_MannequinsXR.ABP_MannequinsXR_C|SetPoseAlphaPoint _asabp_mannequins_xr 0.0))
  (:Canceled
    (goto _label))
  (:Completed
    (bind _asabp_mannequins_xr_2 (Utilities|Casting|CastToABP_MannequinsXR (Components|SkeletalMesh|GetAnimInstance _righthand)))
    (Variables|/Game/LocomotionVR/Characters/MannequinsXR/Meshes/ABP_MannequinsXR.ABP_MannequinsXR_C|SetPoseAlphaPoint _asabp_mannequins_xr_2 1.0)))

(event EventBeginPlay
  (|CallParentFunction)
  (if (Class|HeadMountedDisplayFunctionLibrary|IsHeadMountedDisplayEnabled)
    (Class|HeadMountedDisplayFunctionLibrary|SetTrackingOrigin "Stage")
    (Development|ExecuteConsoleCommand "vr.PixelDensity 1.0" 0)))

(event Collision|EventActorBeginOverlap
  (params (OtherActor :type Actor%20Object%20Reference)))

(event EventTick
  (params (DeltaSeconds :type Float%20%28single-precision%29)))

(fn ConstructionScript)